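; BP_TrackableObject is an actor that visualizes a trackable object as a colored cube.
; UpdateTrackableObjectData sets the actor's transform from the object's center pose and extents, dividing the extents by 50 to convert half extents to cube scale.
; It then looks up the object's label in ObjectColorMap and applies the result to the cube material's Color parameter.
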(event EventBeginPlay)

(event Collision|EventActorBeginOverlap
  (params (OtherActor :type Actor%20Object%20Reference)))

(event EventTick
  (params (DeltaSeconds :type Float%20%28single-precision%29)))

(fn ConstructionScript)

(fn UpdateTrackableObjectData
  (params (Trackable%20Object :type Android%20XR%20Trackable%20Object%20Structure%20%28by%20ref%29))
  (bind (_trackingstate _centerpose _extents _objectlabel) (Utilities|Struct|BreakAndroidXRTrackableObject Trackable%20Object))
  (bind (_x _y _z) (Math|Vector|BreakVector _extents))
  (bind (_location _rotation) (Math|Transform|BreakTransform _centerpose))
  (Utilities|FlowControl|Sequence
    (:then_0
      (Transformation|SetActorTransform (Math|Transform|MakeTransform _location _rotation (Math|Vector|MakeVector (/ _x 5e+01) (/ _y 5e+01) (/ _z 5e+01)))))
    (:then_1
      (bind _objectcolor (CallFunction|SetCubeColor _objectlabel))
      (Rendering|Material|SetColorParameterValueonMaterials (Variables|Default|GetCube) "Color" _objectcolor))))

(fn SetCubeColor
  (params (ObjectLabel :type EAndroidXRTrackablesObjectLabel%20Enum :default "Unknown"))
  (return (.Value (Utilities|Map|Find (Variables|Default|GetObjectColorMap) ObjectLabel))))