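; Actor that displays an Android XR passthrough layer shaped by a static mesh, with opacity, scale and shape editable at runtime.
; Initialize picks the mesh from the game mode's type table, builds the layer from its vertices and triangles, and adds an info widget.
; Widget events are bound to edit or destroy the layer.
; Tick syncs the layer to the mesh transform, optionally easing the actor toward the pawn's MenuTarget.
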(event Custom|ShouldFollowChanged
  (params (ShouldFollow :type Boolean))
  (Variables|Default|SetShouldFollow ShouldFollow))

(event EventBeginPlay
  (bind _asxrgame_mode_passthrough_mesh (Utilities|Casting|CastToXRGameModePassthroughMesh (Game|GetGameMode)))
  (Variables|Default|SetGameMode _asxrgame_mode_passthrough_mesh))

(event Collision|EventActorBeginOverlap
  (params (OtherActor :type Actor%20Object%20Reference)))

(event EventTick
  (params (DeltaSeconds :type Float%20%28single-precision%29))
  (bind _layer (Variables|Default|GetLayer))
  (if (Class|AndroidXRPassthroughMeshBlueprintFunctionLibrary|IsValidPassthroughLayer _layer)
    (Class|AndroidXRPassthroughMeshBlueprintFunctionLibrary|UpdatePassthroughLayerTransform _layer (Transformation|GetWorldTransform (Variables|Default|GetStaticMesh)))
    (if (Variables|Default|GetShouldFollow)
      (bind _position (CallFunction|GetFollowPosition))
      (Transformation|SetActorLocation (Math|Interpolation|VInterpTo (Transformation|GetActorLocation) _position DeltaSeconds 0.0) false false))))

(event EventDestroyed
  (bind _layer (Variables|Default|GetLayer))
  (if (Class|AndroidXRPassthroughMeshBlueprintFunctionLibrary|IsValidPassthroughLayer _layer)
    (Class|AndroidXRPassthroughMeshBlueprintFunctionLibrary|DestroyPassthroughLayer _layer)))

(event EventEndPlay
  (params (EndPlayReason :type EEndPlayReason%20Enum :default "Destroyed"))
  (bind _layer (Variables|Default|GetLayer))
  (if (Class|AndroidXRPassthroughMeshBlueprintFunctionLibrary|IsValidPassthroughLayer _layer)
    (Class|AndroidXRPassthroughMeshBlueprintFunctionLibrary|DestroyPassthroughLayer _layer)))

(fn ConstructionScript)

(fn SetStaticMesh
  (params (MeshType :type String))
  (bind _gamemode (Variables|Default|GetGameMode))
  (bind _meshtypetable (Variables|/Game/XRGameModePassthroughMesh.XRGameModePassthroughMesh_C|GetMeshTypeTable _gamemode))
  (bind (_value _returnvalue) (Utilities|Map|Find _meshtypetable MeshType))
  (if (Utilities|IsValid _gamemode)
    (if _returnvalue
      (Components|StaticMesh|SetStaticMesh (Variables|Default|GetStaticMesh) _value))))

(fn Initialize
  (params (LayerInfo :type Android%20XR%20Passthrough%20Layer%20Mesh%20Info%20Structure%20%28by%20ref%29) (MeshType :type String%20%28by%20ref%29) (MeshInfosUI :type WBP%20Passthrough%20Mesh%20Infos%20Object%20Reference%20%28by%20ref%29))
  (Variables|Default|SetMeshInfosUI MeshInfosUI)
  (CallFunction|SetStaticMesh MeshType)
  (bind (_vertices _triangles) (Class|KismetProceduralMeshLibrary|GetSectionfromStaticMesh (Variables|/Script/Engine.StaticMeshComponent|GetStaticMesh (Variables|Default|GetStaticMesh))))
  (bind (_layer _returnvalue) (Class|AndroidXRPassthroughMeshBlueprintFunctionLibrary|CreatePassthroughLayer (Utilities|Struct|MakeAndroidXRPassthroughLayerMeshInfo (Transformation|GetActorTransform) (.Opacity (Utilities|Struct|BreakAndroidXRPassthroughLayerMeshInfo LayerInfo)) _vertices _triangles)))
  (if _returnvalue
    (Variables|Default|SetLayer _layer)
    (CallFunction|CreateMeshInfoUI MeshType (Utilities|Struct|MakeAndroidXRPassthroughLayerMeshInfo (Transformation|GetActorTransform) (.Opacity (Utilities|Struct|BreakAndroidXRPassthroughLayerMeshInfo LayerInfo)) _vertices _triangles))
    (bind _position (CallFunction|GetFollowPosition))
    (Transformation|SetActorLocation _position false false)))

(fn CreateMeshInfoUI
  (params (MeshType :type String%20%28by%20ref%29) (LayerInfo :type Android%20XR%20Passthrough%20Layer%20Mesh%20Info%20Structure%20%28by%20ref%29))
  (bind _returnvalue (Game|ConstructObjectfromClass "/Game/UMG/PassthroughMesh/WBP_PassthroughMeshInfo.WBP_PassthroughMeshInfo_C"))
  (bind _output_get (Variables|Default|SetMeshInfoUI _returnvalue))
  (Default|AddPassthroughMeshInfo (Variables|Default|GetMeshInfosUI) _output_get)
  (Default|Initialize _output_get MeshType LayerInfo)
  (CallFunction|BindMeshInfoUIEvents))

(fn BindMeshInfoUIEvents
  (bind _meshinfoui (Variables|Default|GetMeshInfoUI))
  (EventDispatchers|BindEventtoOnDestroyLayerClicked _meshinfoui (EventDispatchers|CreateEvent :!event DestroyPassthroughLayer))
  (EventDispatchers|BindEventtoOnOpacityChanged _meshinfoui (EventDispatchers|CreateEvent :!event ChangeLayerOpacity))
  (EventDispatchers|BindEventtoOnScaleChanged _meshinfoui (EventDispatchers|CreateEvent :!event ChangeLayerScale))
  (EventDispatchers|BindEventtoOnMeshShapeChanged _meshinfoui (EventDispatchers|CreateEvent :!event ChangeLayerMesh))
  (EventDispatchers|BindEventtoOnShouldFollowChanged _meshinfoui (EventDispatchers|CreateEvent :!event Custom|ShouldFollowChanged)))

(fn DestroyPassthroughLayer
  (bind _meshinfoui (Variables|Default|GetMeshInfoUI))
  (Class|AndroidXRPassthroughMeshBlueprintFunctionLibrary|DestroyPassthroughLayer (Variables|Default|GetLayer))
  (Default|RemovePassthroughMeshInfo (Variables|Default|GetMeshInfosUI) _meshinfoui)
  (Widget|RemovefromParent _meshinfoui)
  (Actor|DestroyActor))

(fn ChangeLayerOpacity
  (params (Opacity :type Float%20%28double-precision%29))
  (Class|AndroidXRPassthroughMeshBlueprintFunctionLibrary|UpdatePassthroughLayerOpacity (Variables|Default|GetLayer) Opacity))

(fn ChangeLayerMesh
  (params (MeshType :type String%20%28by%20ref%29))
  (bind _gamemode (Variables|Default|GetGameMode))
  (bind _meshtypetable (Variables|/Game/XRGameModePassthroughMesh.XRGameModePassthroughMesh_C|GetMeshTypeTable _gamemode))
  (bind (_value _returnvalue) (Utilities|Map|Find _meshtypetable MeshType))
  (Utilities|IsValid _gamemode
    (:Is%20Valid
      (if _returnvalue
        (Components|StaticMesh|SetStaticMesh (Variables|Default|GetStaticMesh) _value)
        (bind (_vertices _triangles) (Class|KismetProceduralMeshLibrary|GetSectionfromStaticMesh _value))
        (Class|AndroidXRPassthroughMeshBlueprintFunctionLibrary|UpdatePassthroughLayerMesh (Variables|Default|GetLayer) _vertices _triangles)))))

(fn ChangeLayerScale
  (params (Scale :type Float%20%28double-precision%29))
  (Transformation|SetActorScale3D (* Scale "1.000000,1.000000,1.000000")))

(fn GetFollowPosition
  (bind _asxrpawn (Utilities|Casting|CastToXRPawn (Game|Player|GetPlayerPawn 0)))
  (return (Transformation|GetWorldLocation (Variables|/Game/XRPawn.XRPawn_C|GetMenuTarget _asxrpawn))))