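; BP_AnchorSelect is a small, non-colliding visual marker actor, apparently used to show anchor selection.
; On BeginPlay it disables collision, tints its static mesh yellow through a dynamic material instance's Color parameter, and shrinks itself uniformly.
; GetRadius derives a radius from the actor's X scale, assuming a base mesh radius of 50 units.
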(event EventBeginPlay
  (bind _staticmeshcomponent (Variables|Debug|GetStaticMeshComponent))
  (Collision|SetActorEnableCollision false)
  (bind _returnvalue (Rendering|Material|CreateDynamicMaterialInstance (Variables|Debug|GetStaticMeshComponent) 0 (Rendering|Material|GetMaterial _staticmeshcomponent 0) "None" :!class /Script/Engine.PrimitiveComponent))
  (Rendering|Material|SetVectorParameterValue _returnvalue "Color" "(R=0.914286,G=1.000000,B=0.000000,A=1.000000)" :!class /Script/Engine.MaterialInstanceDynamic)
  (Rendering|Material|SetMaterial _staticmeshcomponent 0 _returnvalue)
  (Transformation|SetActorScale3D (Math|Conversions|ToVector(Float) 0.3)))

(event Collision|EventActorBeginOverlap
  (params (OtherActor :type Actor%20Object%20Reference)))

(event EventTick
  (params (DeltaSeconds :type Float%20%28single-precision%29)))

(fn ConstructionScript)

(fn GetRadius
  (return (* (.x (Transformation|GetActorScale3D)) 5e+01)))