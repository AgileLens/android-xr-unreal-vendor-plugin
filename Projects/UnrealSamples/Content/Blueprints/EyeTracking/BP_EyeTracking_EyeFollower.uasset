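; Actor that visualizes Android XR eye tracking with separately colored left and right eye meshes, hidden on BeginPlay.
; UpdateEyeData takes eye data from outside and runs UpdateEye for left, right or both eyes according to its mode.
; A gazing eye's mesh is shown at a fixed distance along that eye's forward vector, while a shut or invalid eye's mesh is hidden.
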(event EventBeginPlay
  (CallFunction|HideEyes)
  (Rendering|Material|SetColorParameterValueonMaterials (Variables|Default|GetRightEye) "Color" (Math|Conversions|ToLinearColor(Color) (Variables|Default|GetRightEyeColor)))
  (Rendering|Material|SetColorParameterValueonMaterials (Variables|Default|GetLeftEye) "Color" (Math|Conversions|ToLinearColor(Color) (Variables|Default|GetLeftEyeColor))))

(event Collision|EventActorBeginOverlap
  (params (OtherActor :type Actor%20Object%20Reference)))

(event EventTick
  (params (DeltaSeconds :type Float%20%28single-precision%29)))

(fn ConstructionScript)

(fn UpdateEyeData
  (params (Eyes :type Android%20XR%20Eyes%20Structure%20%28by%20ref%29))
  (bind (_eyes _mode) (Utilities|Struct|BreakAndroidXREyes Eyes))
  (switch Utilities|FlowControl|Switch|SwitchonEAndroidXREyeTrackingMode _mode
    (:Right
      (CallFunction|UpdateEye (Utilities|Array|Get(acopy) _eyes (Math|Conversions|ToInteger(Byte) (Utilities|Enum|LiteralenumEAndroidXREyeIndex "Right"))) (Variables|Default|GetRightEye) :!label _label))
    (:Left
      (CallFunction|UpdateEye (Utilities|Array|Get(acopy) _eyes (Math|Conversions|ToInteger(Byte) (Utilities|Enum|LiteralenumEAndroidXREyeIndex "Left"))) (Variables|Default|GetLeftEye) :!label _label_2))
    (:Both
      (Utilities|FlowControl|Sequence
        (:then_0
          (goto _label_2))
        (:then_1
          (goto _label))))))

(fn HideEyes
  (Rendering|SetVisibility (Variables|Default|GetLeftEye) false false)
  (Rendering|SetVisibility (Variables|Default|GetRightEye) false false))

(fn ShowEyes
  (Rendering|SetVisibility (Variables|Default|GetRightEye) true false)
  (Rendering|SetVisibility (Variables|Default|GetLeftEye) true false))

(fn UpdateEye
  (params (Eye :type Android%20XR%20Eye%20Structure%20%28by%20ref%29) (Mesh :type Static%20Mesh%20Component%20Object%20Reference%20%28by%20ref%29))
  (bind (_eyestate _transform) (Utilities|Struct|BreakAndroidXREye Eye))
  (bind (_location _rotation) (Math|Transform|BreakTransform _transform))
  (switch Utilities|FlowControl|Switch|SwitchonEAndroidXREyeState _eyestate
    (:Invalid
      (Rendering|SetVisibility Mesh false false :!label _label))
    (:Gazing
      (Rendering|SetVisibility Mesh true false)
      (Transformation|SetWorldLocationAndRotation Mesh (+ _location (* (Math|Vector|RotateVector (Class|KismetMathLibrary|VectorForward) _rotation) 3e+02)) "0, 0, 0" false false))
    (:Shut
      (goto _label))))