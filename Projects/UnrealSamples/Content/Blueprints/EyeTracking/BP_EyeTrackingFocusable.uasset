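; Eye-tracking focusable actor that visually highlights itself when focused and reverts when focus is reset.
; On BeginPlay it caches its initial scale and applies its original color to the static mesh materials.
; FocusObject and ResetFocus, with no caller in this Blueprint, both feed ModifyObject, which sets actor scale and drives the Color and ShouldGlow material parameters.
; Focus multiplies the cached scale by a factor and uses a caller-supplied color.
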(event EventBeginPlay
  (Variables|Default|SetInitialScale (Transformation|GetActorScale3D))
  (Rendering|Material|SetColorParameterValueonMaterials (Variables|Default|GetStaticMesh) "Color" (Math|Conversions|ToLinearColor(Color) (Variables|Default|GetOriginalColor))))

(event Collision|EventActorBeginOverlap
  (params (OtherActor :type Actor%20Object%20Reference)))

(event EventTick
  (params (DeltaSeconds :type Float%20%28single-precision%29)))

(fn ConstructionScript)

(fn FocusObject
  (params (FocusColor :type Color%20Structure%20%28by%20ref%29))
  (CallFunction|ModifyObject (* (Variables|Default|GetInitialScale) (Variables|Default|GetFocusScaleFactor)) FocusColor true))

(fn ResetFocus
  (CallFunction|ModifyObject (Variables|Default|GetInitialScale) (Variables|Default|GetOriginalColor) false))

(fn ModifyObject
  (params (Scale :type Vector%20%28by%20ref%29) (Color :type Color%20Structure%20%28by%20ref%29) (ShouldGlow :type Boolean))
  (bind _staticmesh (Variables|Default|GetStaticMesh))
  (Rendering|Material|SetColorParameterValueonMaterials _staticmesh "Color" (Math|Conversions|ToLinearColor(Color) Color))
  (Transformation|SetActorScale3D Scale)
  (if ShouldGlow
    (LocalVariables|SetGlowValue 1.0)
    (else
      (bind _output_get (LocalVariables|SetGlowValue 0.0))))
  (Rendering|Material|SetScalarParameterValueonMaterials _staticmesh "ShouldGlow" _output_get))