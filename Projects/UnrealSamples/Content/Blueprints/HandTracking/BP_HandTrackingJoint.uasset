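; BP_HandTrackingJoint is a collision-free actor that visualizes a single tracked hand joint.
; An UpdateHandJoint event receives a key point, position, rotation and radius, then moves the actor there and sizes it uniformly by radius times a scale factor.
; An optional text label shows the key point's enum name, or stays empty when labels are off.
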(event EventBeginPlay
  (Collision|SetActorEnableCollision false))

(event Collision|EventActorBeginOverlap
  (params (OtherActor :type Actor%20Object%20Reference)))

(event EventTick
  (params (DeltaSeconds :type Float%20%28single-precision%29)))

(event EventUpdateHandJoint
  (params (HandKeyPoint :type EHandKeypoint%20Enum :default "Palm") (JointPosition :type Vector%20%28by%20ref%29 :default "0, 0, 0") (JointRotation :type Quat%20Structure%20%28by%20ref%29) (JointRadius :type Float%20%28single-precision%29))
  (CallFunction|UpdateHandJointLabel HandKeyPoint)
  (Transformation|SetActorTransform (Math|Transform|MakeTransform JointPosition (Class|KismetMathLibrary|QuatRotator JointRotation) (* (* JointRadius "1.000000,1.000000,1.000000") (Variables|Default|GetScaleFactor)))))

(fn ConstructionScript)

(fn UpdateHandJointLabel
  (params (HandKeyPoint :type EHandKeypoint%20Enum :default "Palm"))
  (bind _textvalue (Variables|Default|GetTextValue))
  (if (Variables|Default|GetbShouldShowLabel)
    (Rendering|Components|TextRender|SetText _textvalue (Utilities|Text|ToText(String) (Utilities|String|EnumtoString HandKeyPoint)))
    (else
      (Rendering|Components|TextRender|SetText _textvalue (Utilities|Text|MakeLiteralText "")))))