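; BP_HandInteraction is a text readout actor that shows a hand interaction type and its readiness, with collision disabled at BeginPlay.
; SetHandInteraction stores the enum, prints its name, and hides the value and ready texts for Poke, Palm and GripSurface, with no path to unhide them.
; SetIsReady colors all three texts green when ready or for those three types, otherwise red.
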(event EventBeginPlay
  (Collision|SetActorEnableCollision false))

(event Collision|EventActorBeginOverlap
  (params (OtherActor :type Actor%20Object%20Reference)))

(event EventTick
  (params (DeltaSeconds :type Float%20%28single-precision%29)))

(fn ConstructionScript)

(fn SetIsReady
  (params (IsReady :type Boolean))
  (bind _handinteraction (Variables|Default|GetHandInteraction))
  (Rendering|Components|TextRender|SetTextRenderColor (Variables|Default|GetTextInteraction) (select (Math|Boolean|ORBoolean IsReady (Utilities|Enum|Equal(Enum) _handinteraction "Poke") (Utilities|Enum|Equal(Enum) _handinteraction "Palm") (Utilities|Enum|Equal(Enum) _handinteraction "GripSurface")) (Math|Color|MakeColor 0 255 0) (Math|Color|MakeColor 0 0 255))))

(fn SetHandInteraction
  (params (HandInteraction :type EOpenXRHandInteractionType%20Enum :default "Aim"))
  (Variables|Default|SetHandInteraction HandInteraction)
  (Rendering|Components|TextRender|SetText (Variables|Default|GetTextInteraction) (Utilities|Text|ToText(String) (Utilities|String|EnumtoString (Variables|Default|GetHandInteraction))))
  (if (Math|Boolean|ORBoolean (Utilities|Enum|Equal(Enum) (Variables|Default|GetHandInteraction) "Poke") (Utilities|Enum|Equal(Enum) (Variables|Default|GetHandInteraction) "Palm") (Utilities|Enum|Equal(Enum) (Variables|Default|GetHandInteraction) "GripSurface"))
    (Development|SetHiddeninGame (Variables|Default|GetTextValue) true false)))